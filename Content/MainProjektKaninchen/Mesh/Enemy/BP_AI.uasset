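; BP_AI is an enemy that roams, then chases and shoots the player on sight, and is destroyed when its health runs out.
; It wanders by re-issuing AIMoveTo to random reachable points after each success.
; PawnSensing reveals its health widget, starts pursuit and immediately turns it to fire Serduszko_pocisk from the "emiter" socket, gated by a cooldown.
; AnyDamage lowers health and updates the widget.
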(event `self.ReceiveBeginPlay`
  (bind _asai_health (cast `/Game/MainProjektKaninchen/Widgets/AI_Health` (`WidgetComponent.GetUserWidgetObject` (`self.Widget`))))
  (set `self.WidgetRef` _asai_health)
  (`self.wANDERINGaROUND`))

(event `self.PawnSensing.OnSeePawn`
  (params (Pawn :type "Pawn Object Reference"))
  (bind _asbp_third_person_character (cast `/Game/MainProjektKaninchen/Mesh/BP_ThirdPersonCharacter` Pawn))
  (set `self.Player` _asbp_third_person_character)
  (`SceneComponent.SetVisibility` (`self.Widget`) true false)
  (`|AIMoveTo` self (0.0 0.0 0.0) (`self.Player`) 1.0
    (:`then`
      (`self.K2_SetActorRotation` (`KismetMathLibrary.FindRelativeLookAtRotation` (`KismetMathLibrary.Conv_VectorToTransform` (`self.K2_GetActorLocation`)) (`self.K2_GetActorLocation` (`self.Player`))))
      (if (`self.Can Attack?`)
        (`|SpawnActorFromClass` "/Game/MainProjektKaninchen/Mesh/Weapon/Serduszko_pocisk.Serduszko_pocisk_C" (`KismetMathLibrary.MakeTransform` (`SceneComponent.GetSocketLocation` (`self.StaticMesh`) "emiter") (`SceneComponent.K2_GetComponentRotation` (`self.SkeletalMesh`))) "Undefined" "OverrideRootScale" null null)
        (set `self.Can Attack?` false)
        (`KismetSystemLibrary.Delay` 1.0)
        (set `self.Can Attack?` true)))))

(event `self.ReceiveAnyDamage`
  (params (Damage :type "Float (single-precision)") (DamageType :type "DamageType Object Reference") (InstigatedBy :type "Controller Object Reference") (DamageCauser :type "Actor Object Reference"))
  (bind _output_get (set `self.Health` (- (`self.Health`) Damage)))
  (set `/Game/MainProjektKaninchen/Widgets/AI_Health.Health` _output_get (`self.WidgetRef`))
  (if (<= _output_get 0.0)
    (`self.K2_DestroyActor`)))

(event `wANDERINGaROUND`
  (`|AIMoveTo` self (`NavigationSystemV1.K2_GetRandomReachablePointInRadius` (`self.K2_GetActorLocation`) 2000.0 null null) null
    (:`OnSuccess`
      (`self.wANDERINGaROUND`))))

(fn `UserConstructionScript`)