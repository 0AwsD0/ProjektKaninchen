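; BP_GameModeKaninchen is the game mode Blueprint that returns the player to their starting point on restart.
; On BeginPlay it caches the player character's location and stores a BP_ThirdPersonCharacter reference.
; Its Restart function teleports the character to that cached location with zero rotation, then calls the character's own Restart.
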(event `self.ReceiveBeginPlay`
  (`self.CashePlayerLocation`)
  (bind _asbp_third_person_character (cast `/Game/MainProjektKaninchen/Mesh/BP_ThirdPersonCharacter` (`GameplayStatics.GetPlayerCharacter` 0)))
  (set `self.Player` _asbp_third_person_character))

(fn `CashePlayerLocation`
  (set `self.Player Location` (`self.K2_GetActorLocation` (`GameplayStatics.GetPlayerCharacter` 0))))

(fn `Restart`
  (`self.K2_TeleportTo` :`self` (`GameplayStatics.GetPlayerCharacter` 0) :`DestLocation` (`self.Player Location`))
  (`/Game/MainProjektKaninchen/Mesh/BP_ThirdPersonCharacter.Restart` (`self.Player`)))

(fn `UserConstructionScript`)